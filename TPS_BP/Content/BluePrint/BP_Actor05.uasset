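; BP_Actor05 is an Actor that scores three dice and prints the result, run once on BeginPlay with hard-coded values.
; The Dice function compares the values for three of a kind, a pair or all different.
; Each case calls its own print function, which computes a score from the matched face, or from the highest die when none match, and shows it via PrintString.
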(event EventBeginPlay
  (CallFunction|Dice 3 3 6))

(fn ConstructionScript)

(fn Dice
  (params (Dice01 :type Integer) (Dice02 :type Integer) (Dice03 :type Integer))
  (Variables|Default|SetDice1 Dice01)
  (Variables|Default|SetDice2 Dice02)
  (Variables|Default|SetDice3 Dice03)
  ;[1 1 1] if : 3개 모두 같은 경우
  (if (and (== (Variables|Default|GetDice1) (Variables|Default|GetDice2)) (== (Variables|Default|GetDice2) (Variables|Default|GetDice3)))
    (CallFunction|PrintEqualThree (Variables|Default|GetDice1))
    (else
      ;[1 1 1] else if : 2개만 같은 경우
      (if (or (== (Variables|Default|GetDice1) (Variables|Default|GetDice2)) (== (Variables|Default|GetDice2) (Variables|Default|GetDice3)))
        (CallFunction|PrintEqualTwo (Variables|Default|GetDice2))
        (elif (== (Variables|Default|GetDice1) (Variables|Default|GetDice3))
          (CallFunction|PrintEqualTwo (Variables|Default|GetDice3))
          (else
            (CallFunction|PrintDifferent (Variables|Default|GetDice1) (Variables|Default|GetDice2) (Variables|Default|GetDice3))))))))

(fn PrintEqualThree
  (params (Dice1 :type Integer))
  (Development|PrintString (Utilities|String|ToString(Integer) (+ (* 1000 Dice1) 10000))))

(fn PrintEqualTwo
  (params (Dice :type Integer))
  (Development|PrintString (Utilities|String|ToString(Integer) (+ (* Dice 100) 1000))))

(fn PrintDifferent
  (params (Dice1 :type Integer) (Dice2 :type Integer) (Dice3 :type Integer))
  (Development|PrintString (Utilities|String|ToString(Integer) (* (Math|Integer|Max(Integer) Dice1 Dice2 Dice3) 100))))