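; BP_Actor07 is an actor that calculates a clock time after adding a number of minutes, then prints the result.
; On BeginPlay it calls Dicision with a hard-coded hour, minute and duration.
; Dicision carries minute overflow into hours with division and modulo, subtracting 24 once if the hour passes midnight.
; It prints the hour, an empty string and the minute as separate messages.
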(event EventBeginPlay
  (CallFunction|Dicision 23 48 25))

(fn ConstructionScript)

(fn Dicision
  (params (a :type Integer) (b :type Integer) (c :type Integer))
  (Variables|Default|Seta a)
  (Variables|Default|Setb b)
  (Variables|Default|Setc c)
  ;[1 1 1] b=b+c
  (bind _output_get (Variables|Default|Setb (+ (Variables|Default|Getb) (Variables|Default|Getc))))
  (if (>= _output_get 60)
    ;[1 1 1] a = a+(b/60)
    (Variables|Default|Seta (+ (Variables|Default|Geta) (/ (Variables|Default|Getb) 60)))
    ;[1 1 1] b=b%60
    (Variables|Default|Setb (Math|Integer|%(Integer) (Variables|Default|Getb) 60))
    (if (>= (Variables|Default|Geta) 24)
      ;[1 1 1] a가 24이상이면 a-=24
      (Variables|Default|Seta (- (Variables|Default|Geta) 24))))
  ;[1 1 1] 시간 분 출력
  (Development|PrintString (Utilities|String|ToString(Integer) (Variables|Default|Geta)))
  (Development|PrintString " ")
  (Development|PrintString (Utilities|String|ToString(Integer) (Variables|Default|Getb))))