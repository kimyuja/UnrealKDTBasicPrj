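; BP_Actor08 is a practice actor that prints the multiplication tables from 2 to 9 as debug text on BeginPlay.
; Two nested loops pair each table number with multipliers 1 through 9 and build each line by appending the operands and product into a string for Print String.
; An unconnected single loop that prints only the 2 times table remains in the graph and never runs.
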(event EventBeginPlay
  ;[1 1 1] 구구단 2~9단
  (for _index (range 2 9)
    (for _index_2 (range 1 9)
      (Development|PrintString (Utilities|String|Append (Utilities|String|ToString(Integer) _index) " * " (Utilities|String|ToString(Integer) _index_2) " = " (Utilities|String|ToString(Integer) (* _index _index_2)))))))

(fn ConstructionScript)