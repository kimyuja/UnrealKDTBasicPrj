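; BP_Actor10 is an actor that prints a five-row star triangle on BeginPlay, apparently a nested-loop exercise.
; Each row builds a padding string and a star string in two inner loops, prints them joined, then clears both.
; The padding loop is meant for leading spaces but appends an empty string as written, so it adds no indentation.
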(event EventBeginPlay
  (for _index (range 1 5)
    ;[1 1 1] 공백 문자열
    (for _index_2 (range 1 (- 5 _index))
      (bind _output_get (Variables|Default|Setspace (Utilities|String|Append (Variables|Default|Getspace) " "))))
    ;[1 1 1] 별 문자열
    (for _index_3 (range 1 _index)
      (bind _output_get_2 (Variables|Default|SetStar (Utilities|String|Append (Variables|Default|GetStar) "*"))))
    (Development|PrintString (Utilities|String|Append _output_get _output_get_2))
    ;[1 1 1] 초기화
    (Variables|Default|SetStar "")
    (Variables|Default|Setspace "")))

(fn ConstructionScript)